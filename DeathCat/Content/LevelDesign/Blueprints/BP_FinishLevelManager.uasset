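; BP_FinishLevelManager ends a level once every enemy in it is killed.
; On BeginPlay it binds to the enemy-killed dispatcher and takes a one-time snapshot of all CharacterAI_Base_BP actors.
; Each kill removes that enemy from the list; when the list empties, it opens the level named by NextLevel, or only prints a game-finished message if that name is None.
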(event Custom|EnemyKilled
  (params (KilledEnemy :type Character%20AI%20Base%20BP%20Object%20Reference))
  (bind _enemylist (Variables|Default|GetEnemyList))
  (bind _nextlevel (Variables|Default|GetNextLevel))
  (Utilities|Array|RemoveItem _enemylist KilledEnemy)
  (if (== (Utilities|Array|Length _enemylist) 0)
    (if (Utilities|Name|Equal(Name) _nextlevel "None")
      (Development|PrintString "GAME FINISHEEEED")
      (else
        (Game|OpenLevel(byName) _nextlevel)))))

(event EventTick
  (params (DeltaSeconds :type Float%20%28single-precision%29)))

(event EventBeginPlay
  (EventDispatchers|BindEventtoEnemyKilledDispatcher (delegate Custom|EnemyKilled))
  (bind _outactors (Actor|GetAllActorsOfClass "/Game/Characters/AI/CharacterAI_Base_BP.CharacterAI_Base_BP_C"))
  (Variables|Default|SetEnemyList _outactors))

(fn ConstructionScript)