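; Moving platform actor that slides back and forth along the world X axis around its placed position.
; On BeginPlay it sets the travel bounds from its start X plus and minus Delta, then keeps tick disabled until StartDelay elapses.
; Each tick moves it by Speed scaled by delta time and flips the Invert direction flag when it reaches either bound, without clamping.
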(event EventBeginPlay
  (bind _returnvalue (Transformation|GetActorLocation))
  (bind _delta (Variables|Default|GetDelta))
  (Variables|Default|SetMaxX (+ (.x _returnvalue) _delta))
  (Variables|Default|SetMinX (- (.x _returnvalue) _delta))
  (Actor|Tick|SetActorTickEnabled false)
  (Utilities|FlowControl|Delay (Variables|Default|GetStartDelay))
  (Actor|Tick|SetActorTickEnabled true))

(event EventTick
  (params (DeltaSeconds :type Float%20%28single-precision%29))
  (bind _returnvalue (Transformation|GetActorLocation))
  (bind _returnvalue_2 (Transformation|GetActorLocation))
  (bind _speed (Variables|Default|GetSpeed))
  (if (Variables|Default|GetInvert)
    (Transformation|SetActorLocation (Math|Vector|MakeVector (+ (* _speed DeltaSeconds) (.x _returnvalue)) (.y _returnvalue) (.z _returnvalue)) false false)
    (else
      (Transformation|SetActorLocation (Math|Vector|MakeVector (- (.x _returnvalue_2) (* _speed DeltaSeconds)) (.y _returnvalue_2) (.z _returnvalue_2)) false false)))
  (if (or (<= (.x _returnvalue) (Variables|Default|GetMinX)) (>= (.x _returnvalue) (Variables|Default|GetMaxX)))
    (Variables|Default|SetInvert (not (Variables|Default|GetInvert)))))

(fn ConstructionScript)