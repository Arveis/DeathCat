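; Falling platform actor that drops its Cube in two stages when anything overlaps its Box trigger.
; The overlap plays a camera shake at the actor's location, then after a short delay moves the Cube down from its cached start position.
; A second delayed move lowers it further, with distance and duration per stage set by variables.
; A second camera shake exists but is unconnected and never runs.
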(event OnComponentBeginOverlap(Box)
  (params (OverlappedComponent :type Primitive%20Component%20Object%20Reference) (OtherActor :type Actor%20Object%20Reference) (OtherComp :type Primitive%20Component%20Object%20Reference) (OtherBodyIndex :type Integer) (bFromSweep :type Boolean) (SweepResult :type Hit%20Result%20Structure%20%28by%20ref%29))
  (bind _cube (Variables|Default|GetCube))
  (bind _beginlocation (Variables|Default|GetBeginLocation))
  (bind _relativelocation (Variables|/Script/Engine.SceneComponent|GetRelativeLocation _cube))
  (Utilities|FlowControl|Sequence
    (:then_0
      (Camera|PlayWorldCameraShake (Variables|Default|GetFirstCameraShake) (Transformation|GetActorLocation self) 1e+03 1e+03))
    (:then_1
      (Utilities|FlowControl|Delay 0.2)
      (Components|MoveComponentTo (Variables|Default|GetCube) (Math|Vector|MakeVector (.x _beginlocation) (.y _beginlocation) (- (.z _beginlocation) (Variables|Default|GetFirstZDifference))) (Variables|Default|GetRotation) false false (Variables|Default|GetFirstFallingTime) false)
      (Utilities|FlowControl|Sequence
        (:then_1
          (Utilities|FlowControl|Delay 0.2)
          (Components|MoveComponentTo (Variables|Default|GetCube) (Math|Vector|MakeVector (.x _relativelocation) (.y _relativelocation) (- (.z _relativelocation) (Variables|Default|GetSecondZDifference))) (Variables|Default|GetRotation) false false (Variables|Default|GetSecondFallingTime) false))))))

(event EventBeginPlay
  (bind _cube (Variables|Default|GetCube))
  (Variables|Default|SetBeginLocation (Variables|/Script/Engine.SceneComponent|GetRelativeLocation _cube))
  (Variables|Default|SetRotation (Variables|/Script/Engine.SceneComponent|GetRelativeRotation _cube)))

(fn ConstructionScript)