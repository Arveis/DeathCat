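; Moving platform that shuttles its static mesh back and forth along a spline.
; Timeline TravelDistance, scaled by spline length, sets the mesh's world location and applies the spline's yaw as relative rotation, with zero pitch and roll.
; On finish, the timeline calls Reverse, which flips playback using MoveForward, recorded from timeline direction through a resettable DoOnce.
; BeginPlay is empty, so this graph does not start the motion itself.
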(event Custom|Reverse
  (bind _staticmesh (Variables|Default|GetStaticMesh))
  (bind _spline (Variables|Default|GetSpline))
  (Utilities|FlowControl|Sequence
    (:then_0
      (goto _label Reset))
    (:then_1
      (if (Variables|Default|GetbMoveForward)
        (bind (_direction _traveldistance) (Timeline|Timeline_0 Reverse)
          (:Update
            (Transformation|SetWorldLocation _staticmesh (Spline|GetLocationatDistanceAlongSpline _spline (* _traveldistance (Spline|GetSplineLength _spline)) "World") false false)
            (Transformation|SetRelativeRotation _staticmesh (Math|Rotator|MakeRotator 0.0 0.0 (.yaw (Spline|GetRotationatDistanceAlongSpline _spline (* _traveldistance (Spline|GetSplineLength _spline)) "World"))) false false)
            (Utilities|FlowControl|DoOnce false :!label _label
              (:Completed
                (Variables|Default|SetbMoveForward (Utilities|Enum|Equal(Enum) _direction "Forward")))))
          (:Finished
            (CallFunction|Reverse)))
        (else
          (Timeline|Timeline_0 Play))))))

(event EventBeginPlay
  (Utilities|FlowControl|Sequence))

(fn ConstructionScript)