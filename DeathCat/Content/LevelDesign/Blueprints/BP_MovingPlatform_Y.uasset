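; Moving platform actor for level design that travels back and forth along the world Y axis around its starting position.
; BeginPlay sets the travel bounds at Delta either side of the start Y.
; Tick moves it by Speed scaled with delta time, in a direction set by Invert, which toggles when either bound is reached or passed, without clamping the position.
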(event EventBeginPlay
  (bind _returnvalue (Transformation|GetActorLocation))
  (bind _delta (Variables|Default|GetDelta))
  (Variables|Default|SetMaxY (+ (.y _returnvalue) _delta))
  (Variables|Default|SetMinY (- (.y _returnvalue) _delta)))

(event EventTick
  (params (DeltaSeconds :type Float%20%28single-precision%29))
  (bind _returnvalue (Transformation|GetActorLocation))
  (bind _returnvalue_2 (Transformation|GetActorLocation))
  (bind _speed (Variables|Default|GetSpeed))
  (if (Variables|Default|GetInvert)
    (Transformation|SetActorLocation (Math|Vector|MakeVector (.x _returnvalue) (+ (* _speed DeltaSeconds) (.y _returnvalue)) (.z _returnvalue)) false false)
    (else
      (Transformation|SetActorLocation (Math|Vector|MakeVector (.x _returnvalue_2) (- (.y _returnvalue_2) (* _speed DeltaSeconds)) (.z _returnvalue_2)) false false)))
  (if (or (<= (.y _returnvalue) (Variables|Default|GetMinY)) (>= (.y _returnvalue) (Variables|Default|GetMaxY)))
    (Variables|Default|SetInvert (not (Variables|Default|GetInvert)))))

(fn ConstructionScript)