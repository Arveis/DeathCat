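; Manager for the Kamienie stone riddle that clears a tree obstacle once every required stone has been delivered.
; It listens for StoneDelivered events, removing matching tags from TagsToObserve until none remain, then destroys the TreesToDisappear actors.
; The solved flag persists in the shared HealthSG save slot, so on BeginPlay an already solved riddle removes the trees immediately instead of binding the event.
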(event Custom|StoneDelivered_Event
  (params (Tag :type Name))
  (bind _tagstoobserve (Variables|Default|GetTagsToObserve))
  (bind _array_element (Utilities|Array|ForEachLoopwithBreak _tagstoobserve)
    (:LoopBody
      (if (Utilities|Name|Equal(Name) _array_element Tag)
        (Utilities|Array|RemoveItem _tagstoobserve Tag)
        (if (== (Utilities|Array|Length _tagstoobserve) 0)
          (Variables|Default|SetRiddleSolved true)
          (CallFunction|DeleteObstacle)
          (bind _returnvalue (SaveGame|DoesSaveGameExist "HealthSG"))
          (if _returnvalue
            (bind _returnvalue_2 (SaveGame|LoadGamefromSlot "HealthSG"))
            (bind _assave_game_bp (Utilities|Casting|CastToSaveGame_BP _returnvalue_2))
            (Variables|/Game/Characters/Blueprints/SaveGame_BP.SaveGame_BP_C|SetKamienieSolved _assave_game_bp true)
            (SaveGame|SaveGametoSlot _assave_game_bp "HealthSG")
            (else
              (bind _returnvalue_3 (SaveGame|CreateSaveGameObject "/Game/Characters/Blueprints/SaveGame_BP.SaveGame_BP_C"))
              (Variables|/Game/Characters/Blueprints/SaveGame_BP.SaveGame_BP_C|SetKamienieSolved _returnvalue_3 true)
              (SaveGame|SaveGametoSlot _returnvalue_3 "HealthSG"))))))))

(event EventBeginPlay
  (bind _returnvalue (SaveGame|DoesSaveGameExist "HealthSG"))
  (if _returnvalue
    (bind _returnvalue_2 (SaveGame|LoadGamefromSlot "HealthSG"))
    (bind _assave_game_bp (Utilities|Casting|CastToSaveGame_BP _returnvalue_2)))
  (if (Variables|/Game/Characters/Blueprints/SaveGame_BP.SaveGame_BP_C|GetKamienieSolved _assave_game_bp)
    (CallFunction|DeleteObstacle)
    (else
      (EventDispatchers|BindEventtoStoneDelivered (delegate Custom|StoneDelivered_Event)))))

(event Collision|EventActorBeginOverlap
  (params (OtherActor :type Actor%20Object%20Reference)))

(event EventTick
  (params (DeltaSeconds :type Float%20%28single-precision%29)))

(fn ConstructionScript)

(fn DeleteObstacle
  (for _array_element (Variables|Default|GetTreesToDisappear)
    (Utilities|IsValid _array_element
      (:Is%20Valid
        (Actor|DestroyActor _array_element)))))