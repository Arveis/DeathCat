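; BP_OpeningTrigger is a level trigger that opens the way by removing assigned obstacles when the player character overlaps it.
; Overlap by a DeathCharacter_BP calls DeleteObstacke, which destroys each valid entry in ItemToDisappear, then the trigger itself.
; BeginPlay runs the same removal immediately if DeletedTrigger is already set.
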(event EventBeginPlay
  (if (Variables|Default|GetDeletedTrigger)
    (CallFunction|DeleteObstacke)))

(event Collision|EventActorBeginOverlap
  (params (OtherActor :type Actor%20Object%20Reference))
  (Utilities|Casting|CastToDeathCharacter_BP OtherActor)
  (CallFunction|DeleteObstacke))

(event EventTick
  (params (DeltaSeconds :type Float%20%28single-precision%29)))

(fn ConstructionScript)

(fn DeleteObstacke
  (bind _result (Utilities|Set|ToArray (Variables|Default|GetItemToDisappear)))
  (for _array_element _result
    (Utilities|IsValid (Utilities|ResolveSoftReference _array_element)
      (:Is%20Valid
        (Actor|DestroyActor (Utilities|ResolveSoftReference _array_element)))))
  (Actor|DestroyActor))