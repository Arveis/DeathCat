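; BP_MovingPlatform_Z is a level-design platform that oscillates vertically around its starting height.
; BeginPlay derives upper and lower Z limits by adding and subtracting Delta from the start position.
; Tick moves the actor along Z at a frame-rate-scaled Speed, with Invert selecting up or down, and flips Invert whenever either limit is reached or passed.
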(event EventBeginPlay
  (bind _returnvalue (Transformation|GetActorLocation))
  (bind _delta (Variables|Default|GetDelta))
  (Variables|Default|SetMaxZ (+ (.z _returnvalue) _delta))
  (Variables|Default|SetMinZ (- (.z _returnvalue) _delta)))

(event EventTick
  (params (DeltaSeconds :type Float%20%28single-precision%29))
  (bind _returnvalue (Transformation|GetActorLocation))
  (bind _returnvalue_2 (Transformation|GetActorLocation))
  (bind _speed (Variables|Default|GetSpeed))
  (if (Variables|Default|GetInvert)
    (Transformation|SetActorLocation (Math|Vector|MakeVector (.x _returnvalue) (.y _returnvalue) (+ (* _speed DeltaSeconds) (.z _returnvalue))) false false)
    (else
      (Transformation|SetActorLocation (Math|Vector|MakeVector (.x _returnvalue_2) (.y _returnvalue_2) (- (.z _returnvalue_2) (* _speed DeltaSeconds))) false false)))
  (if (or (<= (.z _returnvalue) (Variables|Default|GetMinZ)) (>= (.z _returnvalue) (Variables|Default|GetMaxZ)))
    (Variables|Default|SetInvert (not (Variables|Default|GetInvert)))))

(fn ConstructionScript)