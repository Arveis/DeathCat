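; Base Blueprint for AI characters with flipbook sprites that animate by movement and detect their fated item.
; Each tick, axis input sets a four-way facing, favoring vertical over horizontal, which picks the directional flipbook while moving, with idle at zero velocity.
; A sphere overlap with an item stores it as the desired item if its first tag matches the fated tag, otherwise clears it.
; Death destroys the actor.
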(event OnComponentBeginOverlap(Sphere)
  (params (OverlappedComponent :type Primitive%20Component%20Object%20Reference) (OtherActor :type Actor%20Object%20Reference) (OtherComp :type Primitive%20Component%20Object%20Reference) (OtherBodyIndex :type Integer) (bFromSweep :type Boolean) (SweepResult :type Hit%20Result%20Structure%20%28by%20ref%29))
  (bind _asitem_bp (Utilities|Casting|CastToItem_BP OtherActor))
  (if (Utilities|Name|Equal(Name) (Utilities|Array|Get(acopy) (Variables|/Script/Engine.Actor|GetTags _asitem_bp)) (Class|DeathCharacter|GetFatedItemTag))
    (Variables|Default|SetFoundItem true)
    (Variables|Default|SetDesiredItem _asitem_bp)
    (else
      (Variables|Default|SetFoundItem false)
      (Variables|Default|SetDesiredItem 0))))

(event Custom|Die
  (Actor|DestroyActor))

(event EventTick
  (params (DeltaSeconds :type Float%20%28single-precision%29))
  (|CallParentFunction DeltaSeconds)
  (CallFunction|SetDirection))

(fn ConstructionScript)

(fn SetDirection
  (bind _returnvalue (Input|AxisValues|GetYAxis))
  (if (or (!= (Input|AxisValues|GetXAxis) 0.0) (!= (Input|AxisValues|GetYAxis) 0.0))
    (Variables|Default|SetDirection (select (> _returnvalue 0.0) "Up" (select (< _returnvalue 0.0) "Down" (select (> (Input|AxisValues|GetXAxis) 0.0) "Left" "Right")))))
  (Sprite|SetFlipbook (Variables|Default|GetSprite) (select (> (Math|Vector|VectorLength (Transformation|GetVelocity)) 0.0) (Utilities|Select :Index (Variables|Default|GetDirection) :Up (Variables|Default|GetUpAnim) :Down (Variables|Default|GetDownAnim) :Left (Variables|Default|GetLeftAnim) :Right (Variables|Default|GetRightAnim)) (Variables|Default|GetIdleAnimation))))