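; Checkpoint actor that records its own location to a save game when a DeathCharacter enters its sphere trigger.
; On overlap, it loads the existing SaveGame_BP from the HealthSG slot, or creates one if none exists, then sets Location and writes it back to that slot.
; Updating the loaded object keeps any other data already saved in the slot.
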(event OnComponentBeginOverlap(Sphere)
  (params (OverlappedComponent :type Primitive%20Component%20Object%20Reference) (OtherActor :type Actor%20Object%20Reference) (OtherComp :type Primitive%20Component%20Object%20Reference) (OtherBodyIndex :type Integer) (bFromSweep :type Boolean) (SweepResult :type Hit%20Result%20Structure%20%28by%20ref%29))
  (bind _returnvalue (Transformation|GetActorLocation))
  (Utilities|Casting|CastToDeathCharacter OtherActor)
  (bind _returnvalue_2 (SaveGame|DoesSaveGameExist "HealthSG"))
  (if _returnvalue_2
    (bind _returnvalue_3 (SaveGame|LoadGamefromSlot "HealthSG"))
    (bind _assave_game_bp (Utilities|Casting|CastToSaveGame_BP _returnvalue_3))
    (Variables|/Game/Characters/Blueprints/SaveGame_BP.SaveGame_BP_C|SetLocation _assave_game_bp _returnvalue)
    (SaveGame|SaveGametoSlot _assave_game_bp "HealthSG")
    (else
      (bind _returnvalue_4 (SaveGame|CreateSaveGameObject "/Game/Characters/Blueprints/SaveGame_BP.SaveGame_BP_C"))
      (Variables|/Game/Characters/Blueprints/SaveGame_BP.SaveGame_BP_C|SetLocation _returnvalue_4 _returnvalue)
      (SaveGame|SaveGametoSlot _returnvalue_4 "HealthSG"))))

(event EventBeginPlay)

(event Collision|EventActorBeginOverlap
  (params (OtherActor :type Actor%20Object%20Reference)))

(event EventTick
  (params (DeltaSeconds :type Float%20%28single-precision%29)))

(fn ConstructionScript)