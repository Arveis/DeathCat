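; CharacterAI_Base_BP is a base AI character Blueprint that drives directional 2D flipbook animation for its sprite.
; Each tick, after the parent tick, SetDirection derives a four-way facing from the X and Y axis values, with Y taking priority and positive X mapping to Left.
; The last facing persists without axis input and selects the flipbook while velocity is nonzero, otherwise the idle animation plays.
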(event EventTick
  (params (DeltaSeconds :type Float%20%28single-precision%29))
  (|CallParentFunction DeltaSeconds)
  (CallFunction|SetDirection))

(fn ConstructionScript)

(fn SetDirection
  (bind _returnvalue (Input|AxisValues|GetYAxis))
  (if (or (!= (Input|AxisValues|GetXAxis) 0.0) (!= (Input|AxisValues|GetYAxis) 0.0))
    (Variables|Default|SetDirection (select (> _returnvalue 0.0) "Up" (select (< _returnvalue 0.0) "Down" (select (> (Input|AxisValues|GetXAxis) 0.0) "Left" "Right")))))
  (Sprite|SetFlipbook (Variables|Default|GetSprite) (select (> (Math|Vector|VectorLength (Transformation|GetVelocity)) 0.0) (Utilities|Select :Index (Variables|Default|GetDirection) :Up (Variables|Default|GetUpAnim) :Down (Variables|Default|GetDownAnim) :Left (Variables|Default|GetLeftAnim) :Right (Variables|Default|GetRightAnim)) (Variables|Default|GetIdleAnimation))))