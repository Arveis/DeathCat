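; Pickup item actor that the player character (DeathCharacter_BP) collects into an Items array, with optional two-item combining.
; BeginPlay applies the sprite from the item struct, and a trigger overlap toggles input while the player is in range.
; On Action press, it swaps a held SecondItemBP for NewItem, or otherwise adds itself.
; The collected actor is moved far below via relative location rather than destroyed.
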(event OnComponentBeginOverlap(Trigger)
  (params (OverlappedComponent :type Primitive%20Component%20Object%20Reference) (OtherActor :type Actor%20Object%20Reference) (OtherComp :type Primitive%20Component%20Object%20Reference) (OtherBodyIndex :type Integer) (bFromSweep :type Boolean) (SweepResult :type Hit%20Result%20Structure%20%28by%20ref%29))
  ;[1 1 1] Is player in range
  (Utilities|Casting|CastToDeathCharacter_BP OtherActor)
  (Variables|Default|SetIsInRange true)
  (Input|EnableInput (Game|GetPlayerController 0)))

(event OnComponentEndOverlap(Trigger)
  (params (OverlappedComponent :type Primitive%20Component%20Object%20Reference) (OtherActor :type Actor%20Object%20Reference) (OtherComp :type Primitive%20Component%20Object%20Reference) (OtherBodyIndex :type Integer))
  ;[1 1 1] Is player in range
  (Utilities|Casting|CastToDeathCharacter_BP OtherActor)
  (Variables|Default|SetIsInRange false)
  (Input|DisableInput (Game|GetPlayerController 0)))

(event EventBeginPlay
  ;[1 1 1] Set Sprite at BeginPlay
  (Rendering|Components|Sprite|SetSprite (Variables|Default|GetItemSprite) (.sprite (Variables|Setup|GetItemStruct))))

(event Collision|EventActorBeginOverlap
  (params (OtherActor :type Actor%20Object%20Reference)))

(event EventTick
  (params (DeltaSeconds :type Float%20%28single-precision%29)))

(event Input|ActionEvents|InputActionAction
  (params (Key :type Key%20Structure :default "None"))
  (bind _returnvalue (Game|GetPlayerController 0))
  (bind _seconditembp (Variables|Setup|GetSecondItemBP))
  ;[1 1 1] PickUp item and combine if possible
  (:Pressed
    (if (Variables|Default|GetIsInRange)
      (bind _asdeath_character_bp (Utilities|Casting|CastToDeathCharacter_BP (Game|GetPlayerCharacter 0)))
      (if (and (Utilities|IsValid (Variables|Setup|GetSecondItemBP)) (Utilities|IsValid (Variables|Setup|GetNewItem)))
        (for (_array_element _array_index) (Variables|/Game/Characters/Blueprints/DeathCharacter_BP.DeathCharacter_BP_C|GetItems _asdeath_character_bp)
          (if (== _array_element _seconditembp)
            (Variables|Default|SetIsSecondItemHere true)
            (Variables|Default|SetSecondIndex _array_index)))
        (if (Variables|Default|GetIsSecondItemHere)
          (Variables|Default|SetIsSecondItemHere false)
          (Utilities|Array|RemoveItem (Variables|/Game/Characters/Blueprints/DeathCharacter_BP.DeathCharacter_BP_C|GetItems _asdeath_character_bp) _seconditembp)
          (Utilities|Array|AddUnique (Variables|/Game/Characters/Blueprints/DeathCharacter_BP.DeathCharacter_BP_C|GetItems _asdeath_character_bp) (Variables|Setup|GetNewItem))
          (Input|DisableInput _returnvalue)
          (Transformation|SetActorRelativeLocation "0, 0,-1000.000000")
          (else
            (Utilities|Array|AddUnique (Variables|/Game/Characters/Blueprints/DeathCharacter_BP.DeathCharacter_BP_C|GetItems _asdeath_character_bp) self :!label _label)
            (Input|DisableInput _returnvalue)
            (Transformation|SetActorRelativeLocation "0, 0,-1000.000000")))
        (else
          (goto _label))))))

(fn ConstructionScript)